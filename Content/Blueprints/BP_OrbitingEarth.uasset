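; BP_OrbitingEarth is an animated Earth actor that orbits on an arm, with cloud and atmosphere layers and a separate Moon orbit arm.
; Tick applies delta-time-scaled local yaw to each component, so motion is frame-rate independent.
; The orbit arm turns slowly, Earth and atmosphere spin together, clouds drift slightly faster, and the Moon arm rotates fastest.
; BeginPlay, overlap and the construction script are empty.
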(event EventBeginPlay)

(event Collision|EventActorBeginOverlap
  (params (OtherActor :type Actor%20Object%20Reference)))

(event EventTick
  (params (DeltaSeconds :type Float%20%28single-precision%29))
  (bind _returnvalue (* DeltaSeconds 6e+01))
  (bind _returnvalue_2 (Math|Rotator|MakeRotator 0.0 0.0 _returnvalue))
  (Transformation|AddLocalRotation (Variables|Default|GetOrbitArm) (Math|Rotator|MakeRotator 0.0 0.0 (* DeltaSeconds 8.0)) false false)
  (Transformation|AddLocalRotation (Variables|Default|GetEarth_Mesh) _returnvalue_2 false false)
  (Transformation|AddLocalRotation (Variables|Default|GetEarth_Cloud_Mesh) (Math|Rotator|MakeRotator 0.0 0.0 (* DeltaSeconds 7e+01)) false false)
  (Transformation|AddLocalRotation (Variables|Default|GetEarth_Atmophere_Mesh) _returnvalue_2 false false)
  (Transformation|AddLocalRotation (Variables|Default|GetMoonOrbitArm) (Math|Rotator|MakeRotator 0.0 0.0 (* DeltaSeconds 8e+01)) false false))

(fn ConstructionScript)