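; Solar system actor that animates the orbit and spin of Mercury, Venus and Mars through Neptune, with no Earth in its logic.
; BeginPlay sets each planet's orbit arm to a fixed starting yaw to stagger the planets.
; Tick adds frame-rate-independent local yaw to each orbit arm and planet mesh at hardcoded per-planet speeds.
; Venus has a separate atmosphere component that spins at the same rate as its mesh.
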(event EventBeginPlay
  (Transformation|SetRelativeRotation (Variables|Default|GetMercury_OrbitArm) "0.000000,20.000000,0.000000" false false)
  (Transformation|SetRelativeRotation (Variables|Default|GetVenus_OrbitArm) "0.000000,80.000000,0.000000" false false)
  (Transformation|SetRelativeRotation (Variables|Default|GetJupiter_OrbitArm) "0.000000,300.000000,0.000000" false false)
  (Transformation|SetRelativeRotation (Variables|Default|GetSaturn_OrbitArm) "0.000000,40.000000,0.000000" false false)
  (Transformation|SetRelativeRotation (Variables|Default|GetUranus_OrbitArm) "0.000000,120.000000,0.000000" false false)
  (Transformation|SetRelativeRotation (Variables|Default|GetNeptune_OrbitArm) "0.000000,210.000000,0.000000" false false)
  (Transformation|SetRelativeRotation (Variables|Default|GetMars_OrbitArm) "0.000000,230.000000,0.000000" false false))

(event EventTick
  (params (DeltaSeconds :type Float%20%28single-precision%29))
  (Transformation|AddLocalRotation (Variables|Default|GetMars_OrbitArm) (Math|Rotator|MakeRotator 0.0 0.0 (* DeltaSeconds 6.0)) false false)
  (Transformation|AddLocalRotation (Variables|Default|GetMars_Mesh) (Math|Rotator|MakeRotator 0.0 0.0 (* DeltaSeconds 59.0)) false false)
  (Transformation|AddLocalRotation (Variables|Default|GetJupiter_OrbitArm) (Math|Rotator|MakeRotator 0.0 0.0 (* DeltaSeconds 3.0)) false false)
  (Transformation|AddLocalRotation (Variables|Default|GetJupiter_Mesh) (Math|Rotator|MakeRotator 0.0 0.0 (* DeltaSeconds 9e+01)) false false)
  (Transformation|AddLocalRotation (Variables|Default|GetSaturn_OrbitArm) (Math|Rotator|MakeRotator 0.0 0.0 (* DeltaSeconds 2.0)) false false)
  (Transformation|AddLocalRotation (Variables|Default|GetSaturn_Mesh) (Math|Rotator|MakeRotator 0.0 0.0 (* DeltaSeconds 75.0)) false false)
  (Transformation|AddLocalRotation (Variables|Default|GetUranus_OrbitArm) (Math|Rotator|MakeRotator 0.0 0.0 (* DeltaSeconds 1.3)) false false)
  (Transformation|AddLocalRotation (Variables|Default|GetUranus_Mesh) (Math|Rotator|MakeRotator 0.0 0.0 (* DeltaSeconds 5e+01)) false false)
  (Transformation|AddLocalRotation (Variables|Default|GetNeptune_OrbitArm) (Math|Rotator|MakeRotator 0.0 0.0 (* DeltaSeconds 1.0)) false false)
  (Transformation|AddLocalRotation (Variables|Default|GetNeptune_Mesh) (Math|Rotator|MakeRotator 0.0 0.0 (* DeltaSeconds 55.0)) false false)
  (Transformation|AddLocalRotation (Variables|Default|GetVenus_OrbitArm) (Math|Rotator|MakeRotator 0.0 0.0 (* DeltaSeconds 1e+01)) false false)
  (Transformation|AddLocalRotation (Variables|Default|GetVenus_Mesh) (Math|Rotator|MakeRotator 0.0 0.0 (* DeltaSeconds 2e+01)) false false)
  (Transformation|AddLocalRotation (Variables|Default|GetVenus_Atmosphere) (Math|Rotator|MakeRotator 0.0 0.0 (* DeltaSeconds 2e+01)) false false)
  (Transformation|AddLocalRotation (Variables|Default|GetMercury_OrbitArm) (Math|Rotator|MakeRotator 0.0 0.0 (* 14.0 DeltaSeconds)) false false)
  (Transformation|AddLocalRotation (Variables|Default|GetMercury_Mesh) (Math|Rotator|MakeRotator 0.0 0.0 (* 25.0 DeltaSeconds)) false false))

(fn ConstructionScript)